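; Player controller for the skill test that turns Enhanced Input actions into actions on the controlled pawn.
; On possess it adds the game mapping context, then handles yaw-relative movement and look with sensitivity and optional pitch inversion.
; Sprint switches the base character's walk speed between sprint and run, and crouch toggles.
; Fire input drives a BP_Phase pawn's projectile through spawn, cancel and launch, printing each state as debug text.
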(event `self.ReceivePossess`
  (params (PossessedPawn :type "Pawn Object Reference"))
  (bind _returnvalue (subsystem `EnhancedInputLocalPlayerSubsystem`))
  (`/Engine/EditorBlueprintResources/StandardMacros.IsValid` _returnvalue
    (:`Is Valid`
      (`EnhancedInputSubsystemInterface.AddMappingContext` _returnvalue "/Game/_GameManager/Inputs/IMC_Game.IMC_Game" 0 (struct)))))

(event `EnhancedInput|/Game/_GameManager/Inputs/IA_Move`
  (params (ActionValue :type "Vector2D Structure") (ElapsedSeconds :type "Float (double-precision)") (TriggeredSeconds :type "Float (double-precision)") (InputAction :type "InputAction Object Reference" :default "/Game/_GameManager/Inputs/IA_Move.IA_Move"))
  (bind (_x _y) (`KismetMathLibrary.BreakVector2D` ActionValue))
  (bind (_returnvalue_roll _returnvalue_pitch _returnvalue_yaw) (`KismetMathLibrary.BreakRotator` (`self.GetControlRotation`)))
  (bind _returnvalue (`KismetMathLibrary.MakeRotator` _returnvalue_roll 0.0 _returnvalue_yaw))
  (:`Triggered`
    (`Pawn.AddMovementInput` (`self.K2_GetPawn`) (`KismetMathLibrary.GetForwardVector` _returnvalue) _y false) ; Forward
    (`Pawn.AddMovementInput` (`self.K2_GetPawn`) (`KismetMathLibrary.GetRightVector` _returnvalue) _x false) ; Right
  ))

(event `EnhancedInput|/Game/_GameManager/Inputs/IA_Sprint`
  (params (ActionValue :type Boolean) (ElapsedSeconds :type "Float (double-precision)") (TriggeredSeconds :type "Float (double-precision)") (InputAction :type "InputAction Object Reference" :default "/Game/_GameManager/Inputs/IA_Sprint.IA_Sprint"))
  (bind _asbp_base_character (cast `/Game/_GameManager/BP_BaseCharacter` (`self.K2_GetPawn`) :!pure true))
  (bind _asbp_base_character_2 (cast `/Game/_GameManager/BP_BaseCharacter` (`self.K2_GetPawn`) :!pure true))
  (:`Started`
    (set `CharacterMovementComponent.MaxWalkSpeed` (`/Game/_GameManager/BP_BaseCharacter.SprintSpeed` _asbp_base_character_2) (`Character.CharacterMovement` _asbp_base_character_2)) ; Sprint
  )
  (:`Completed`
    (set `CharacterMovementComponent.MaxWalkSpeed` (`/Game/_GameManager/BP_BaseCharacter.RunSpeed` _asbp_base_character) (`Character.CharacterMovement` _asbp_base_character)) ; Run
  ))

(event `EnhancedInput|/Game/_GameManager/Inputs/IA_Crouch`
  (params (ActionValue :type Boolean) (ElapsedSeconds :type "Float (double-precision)") (TriggeredSeconds :type "Float (double-precision)") (InputAction :type "InputAction Object Reference" :default "/Game/_GameManager/Inputs/IA_Crouch.IA_Crouch"))
  (bind _ascharacter (cast `Character` (`self.K2_GetPawn`) :!pure true))
  (:`Started`
    (if (`Character.bIsCrouched` _ascharacter)
      (`Character.UnCrouch` _ascharacter)
      (else
        (`Character.Crouch` _ascharacter)))))

(event `EnhancedInput|/Game/_GameManager/Inputs/IA_Look`
  (params (ActionValue :type "Vector2D Structure") (ElapsedSeconds :type "Float (double-precision)") (TriggeredSeconds :type "Float (double-precision)") (InputAction :type "InputAction Object Reference" :default "/Game/_GameManager/Inputs/IA_Look.IA_Look"))
  (bind (_x _y) (`KismetMathLibrary.BreakVector2D` (* ActionValue (`self.Sensibility`))))
  (:`Triggered`
    (`self.AddYawInput` _x)
    (`self.AddPitchInput` (* _y (`KismetMathLibrary.SelectFloat` -1.0 1.0 (`self.InvertCamera`))))))

(event `EnhancedInput|/Game/_GameManager/Inputs/IA_FireProjectile`
  (params (ActionValue :type Boolean) (ElapsedSeconds :type "Float (double-precision)") (TriggeredSeconds :type "Float (double-precision)") (InputAction :type "InputAction Object Reference" :default "/Game/_GameManager/Inputs/IA_FireProjectile.IA_FireProjectile"))
  (:`Started`
    (`KismetSystemLibrary.PrintString` "Started")
    (bind _asbp_phase (cast `/Game/Characters/BP_Phase` (`self.K2_GetPawn`)))
    (`/Game/Characters/BP_Phase.SpawnProjectile` _asbp_phase))
  (:`Canceled`
    (`KismetSystemLibrary.PrintString` "Canceled")
    (bind _asbp_phase_2 (cast `/Game/Characters/BP_Phase` (`self.K2_GetPawn`)))
    (`/Game/Characters/BP_Phase.CancelProjectile` _asbp_phase_2))
  (:`Completed`
    (`KismetSystemLibrary.PrintString` "Completed")
    (bind _asbp_phase_3 (cast `/Game/Characters/BP_Phase` (`self.K2_GetPawn`)))
    (`/Game/Characters/BP_Phase.LaunchProjectile` _asbp_phase_3)))

(fn `UserConstructionScript`)