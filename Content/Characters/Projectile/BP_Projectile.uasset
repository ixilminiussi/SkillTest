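; Projectile actor that flies along the firing pawn's aim and damages whatever it hits, apart from BP_Phase characters.
; ShootProjectile sets velocity from control rotation at max speed, then after a short lifetime delay destroys the actor and stops the BP_Phase shooter's stored camera shake.
; A valid hit spawns an impact Niagara effect, plays a light radial camera shake, applies damage and destroys the projectile.
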(event `ShootProjectile`
  (params (Pawn :type "Pawn Object Reference"))
  (bind _projectilemovement (`self.ProjectileMovement`))
  (set `MovementComponent.Velocity` (* (`KismetMathLibrary.GetForwardVector` (`Pawn.GetControlRotation` Pawn)) (`ProjectileMovementComponent.MaxSpeed` _projectilemovement)) _projectilemovement)
  (`KismetSystemLibrary.Delay` 3.0)
  (`self.K2_DestroyActor`)
  (bind _asbp_phase (cast `/Game/Characters/BP_Phase` Pawn))
  (`PlayerCameraManager.StopCameraShake` (`GameplayStatics.GetPlayerCameraManager` 0) (`/Game/Characters/BP_Phase.ShakeSource` _asbp_phase) true))

(event `self.ReceiveHit`
  (params (MyComp :type "PrimitiveComponent Object Reference") (Other :type "Actor Object Reference") (OtherComp :type "PrimitiveComponent Object Reference") (bSelfMoved :type Boolean) (HitLocation :type "Vector Structure") (HitNormal :type "Vector Structure") (NormalImpulse :type "Vector Structure") (Hit :type "HitResult Structure (by ref)"))
  (cast `/Game/Characters/BP_Phase` Other
    (:`CastFailed`
      (`NiagaraFunctionLibrary.SpawnSystemAtLocation` "/Game/Characters/Projectile/NS_Projectile_Impact.NS_Projectile_Impact" HitLocation)
      (`GameplayStatics.PlayWorldCameraShake` "/Game/Characters/Projectile/BP_CameraShake_Light.BP_CameraShake_Light_C" (`self.K2_GetActorLocation`) 1000.0 2500.0 1.0 true)
      (`GameplayStatics.ApplyDamage` Other 10.0)
      (`self.K2_DestroyActor`))))

(fn `UserConstructionScript`)