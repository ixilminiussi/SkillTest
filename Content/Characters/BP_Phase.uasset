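; BP_Phase is a character Blueprint that manages the spawn, cancel and launch of a projectile attack.
; SpawnProjectile creates a BP_Projectile, stores it and attaches it to the mesh's ProjectileSocket.
; CancelProjectile destroys the stored projectile, while LaunchProjectile detaches it in world space and calls its ShootProjectile, passing itself.
; The construction script only calls the parent's.
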(event `SpawnProjectile`
  (bind _returnvalue (`|SpawnActorFromClass` "/Game/Characters/BP_Projectile.BP_Projectile_C" (`KismetMathLibrary.MakeTransform` (0.0 0.0 0.0)) "Undefined" "MultiplyWithRoot" null null))
  (bind _output_get (set `self.Projectile` _returnvalue))
  (`self.K2_AttachToComponent` _output_get (`self.Mesh`) "ProjectileSocket" "KeepRelative" "KeepRelative" "KeepRelative" true))

(event `CancelProjectile`
  (`self.K2_DestroyActor` (`self.Projectile`)))

(event `LaunchProjectile`
  (`self.K2_DetachFromActor` (`self.Projectile`) "KeepWorld" "KeepWorld" "KeepWorld")
  (`/Game/Characters/BP_Projectile.ShootProjectile` (`self.Projectile`) self))

(fn `UserConstructionScript`
  (`parent.UserConstructionScript`))